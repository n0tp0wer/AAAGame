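; Usable actor that shows an interaction prompt on the player's HUD text while focused.
; StartFocusItem displays "Press E to interact" through FPSCharacter_BP, and EndFocusItem blanks it, both returning true once the cast of player 0's character succeeds.
; The Destroyed event also blanks the text, so the prompt does not linger after the actor is removed.
; No interaction logic lives in this Blueprint.
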(event `self.ReceiveDestroyed`
  (bind _asfpscharacter_bp (cast `/Game/Blueprints/FPSCharacter_BP` (`GameplayStatics.GetPlayerCharacter` 0)))
  (`/Game/Blueprints/FPSCharacter_BP.TextBackToBlank` _asfpscharacter_bp))

(fn `EndFocusItem`
  (returns (ReturnValue :type Boolean))
  (bind _asfpscharacter_bp (cast `/Game/Blueprints/FPSCharacter_BP` (`GameplayStatics.GetPlayerCharacter` 0)))
  (`/Game/Blueprints/FPSCharacter_BP.TextBackToBlank` _asfpscharacter_bp)
  (return true))

(fn `StartFocusItem`
  (returns (ReturnValue :type Boolean))
  (bind _asfpscharacter_bp (cast `/Game/Blueprints/FPSCharacter_BP` (`GameplayStatics.GetPlayerCharacter` 0)))
  (`/Game/Blueprints/FPSCharacter_BP.DisplayInstructionText` _asfpscharacter_bp "Press E to interact")
  (return true))

(fn `UserConstructionScript`)