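; Game mode that respawns the player's FPS character after it is destroyed and tracks a list of items to find.
; On BeginPlay it binds to the character's OnDestroyed, then after a short delay spawns a replacement at SpawnPoint, has player controller 0 possess it, and rebinds through Respawn.
; MarkFound looks up the unfound entry by name in ItemsToFind and overwrites it as found.
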(event `Respawn`
  (bind _asfpscharacter_bp (cast `/Game/Blueprints/FPSCharacter_BP` (`GameplayStatics.GetPlayerCharacter` 0) :!label _label))
  (add `self.OnDestroyed` _asfpscharacter_bp (delegate `CustomEvent_0`)))

(event `self.ReceiveBeginPlay`
  (goto _label))

(event `CustomEvent_0` :!signature `self.OnDestroyed`
  (params (DestroyedActor :type "Actor Object Reference"))
  (`KismetSystemLibrary.Delay` 3.0)
  (bind _returnvalue (`|SpawnActorFromClass` "/Game/Blueprints/FPSCharacter_BP.FPSCharacter_BP_C" (`self.SpawnPoint`) "Undefined" "OverrideRootScale" null null))
  (`Controller.Possess` (`GameplayStatics.GetPlayerController` 0) _returnvalue)
  (`self.Respawn`))

(fn `MarkFound`
  (params (Item :type Text))
  (bind _itemstofind (`self.ItemsToFind`))
  (`KismetArrayLibrary.Array_Set` _itemstofind (`KismetArrayLibrary.Array_Find` _itemstofind (make `/Game/Ui/FindList/ItemToFind` false Item)) (make `/Game/Ui/FindList/ItemToFind` true Item)))

(fn `UserConstructionScript`)